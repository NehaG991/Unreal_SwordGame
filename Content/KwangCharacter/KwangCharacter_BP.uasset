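; Player character Blueprint for Kwang that handles sprinting, blocking and a three-hit melee attack combo.
; Sprint input switches the walk speed, and Block input toggles a blocking flag.
; Attack input plays the next of three montages in a cycle, or buffers the press if an attack is already running.
; Combo_Attack consumes the buffered press to chain the next montage, and Attack_End resets the combo state.
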(event Custom|Attack_End
  ;[1 1 1] Combo Functionality
  (Variables|Default|SetattackNumber 0)
  (Variables|Default|SetisAttacking false)
  (Variables|Default|SetsaveAttack false))

(event Custom|Combo_Attack
  ;[1 1 1] Combo Functionality
  (if (Variables|Default|GetsaveAttack)
    (Variables|Default|SetsaveAttack false)
    (switch int (Variables|Default|GetattackNumber)
      (:0
        (Variables|Default|SetattackNumber 1)
        (Animation|PlayAnimMontage "/Game/KwangCharacter/Animations/AttackA_Montage.AttackA_Montage" 1.0 "None"))
      (:1
        (Variables|Default|SetattackNumber 2)
        (Animation|PlayAnimMontage "/Game/KwangCharacter/Animations/AttackB_Montage.AttackB_Montage" 1.0 "None"))
      (:2
        (Variables|Default|SetattackNumber 0)
        (Animation|PlayAnimMontage "/Game/KwangCharacter/Animations/AttackC_Montage.AttackC_Montage" 1.0 "None")))))

(event EventBeginPlay)

(event Collision|EventActorBeginOverlap
  (params (OtherActor :type Actor%20Object%20Reference)))

(event EventTick
  (params (DeltaSeconds :type Float%20%28single-precision%29)))

(event Input|ActionEvents|InputActionBlock
  (params (Key :type Key%20Structure :default "None"))
  ;[1 1 1] Block Fuctionality
  (:Pressed
    (Variables|Default|SetisBlocking true))
  (:Released
    (Variables|Default|SetisBlocking false)))

(event Input|ActionEvents|InputActionAttack
  (params (Key :type Key%20Structure :default "None"))
  ;[1 1 1] Combo Functionality
  (:Pressed
    (if (Variables|Default|GetisAttacking)
      (Variables|Default|SetsaveAttack true)
      (else
        (Variables|Default|SetisAttacking true)
        (switch int (Variables|Default|GetattackNumber)
          (:0
            (Variables|Default|SetattackNumber 1)
            (Animation|PlayAnimMontage "/Game/KwangCharacter/Animations/AttackA_Montage.AttackA_Montage" 1.0 "None"))
          (:1
            (Variables|Default|SetattackNumber 2)
            (Animation|PlayAnimMontage "/Game/KwangCharacter/Animations/AttackB_Montage.AttackB_Montage" 1.0 "None"))
          (:2
            (Variables|Default|SetattackNumber 0)
            (Animation|PlayAnimMontage "/Game/KwangCharacter/Animations/AttackC_Montage.AttackC_Montage" 1.0 "None")))))))

(event Input|ActionEvents|InputActionSprint
  (params (Key :type Key%20Structure :default "None"))
  (bind _charactermovement (Variables|Character|GetCharacterMovement))
  (:Pressed
    (Variables|/Script/Engine.CharacterMovementComponent|SetMaxWalkSpeed _charactermovement 1e+03))
  (:Released
    (Variables|/Script/Engine.CharacterMovementComponent|SetMaxWalkSpeed _charactermovement 5e+02)))

(fn ConstructionScript)